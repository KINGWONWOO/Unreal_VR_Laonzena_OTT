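; BP_CheerStick1 is a grabbable VR cheer stick whose light the player toggles with the holding hand's shoot input.
; Grabbing enables input and adds that hand's weapon mapping context, and dropping reverses both.
; Each press flips IsLightOn, sets Brightness in the shared MPC_CheerStick parameter collection, and plays the pistol-fire haptic on that hand.
; Brightness lives in the collection, so it applies globally rather than per instance.
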(event `EnhancedInput|/Game/ExternalAsset/VRTemplate/Input/Actions/IA_Shoot_Left`
  (params (ActionValue :type Boolean) (ElapsedSeconds :type "Float (double-precision)") (TriggeredSeconds :type "Float (double-precision)") (InputAction :type "InputAction Object Reference" :default "/Game/ExternalAsset/VRTemplate/Input/Actions/IA_Shoot_Left.IA_Shoot_Left"))
  (:`Started`
    (if (`|EnumEquality` (`/Game/ExternalAsset/VRTemplate/Blueprints/GrabComponent.GetHeldByHand` (`self.GrabComponent`)) "Left")
      (if (`self.IsLightOn`) :!label _label
        (set `self.IsLightOn` false)
        (`KismetMaterialLibrary.SetScalarParameterValue` "/Game/Mesh/MPC_CheerStick.MPC_CheerStick" "Brightness")
        (else
          (set `self.IsLightOn` true)
          (`KismetMaterialLibrary.SetScalarParameterValue` "/Game/Mesh/MPC_CheerStick.MPC_CheerStick" "Brightness" 4.0)))
      (`PlayerController.PlayHapticEffect` (`GameplayStatics.GetPlayerController` 0) (`self.PistolFireHapticEffect`) (`/Game/ExternalAsset/VRTemplate/Blueprints/GrabComponent.GetHeldByHand` (`self.GrabComponent`)) 1.0 false))))

(event `EnhancedInput|/Game/ExternalAsset/VRTemplate/Input/Actions/IA_Shoot_Right`
  (params (ActionValue :type Boolean) (ElapsedSeconds :type "Float (double-precision)") (TriggeredSeconds :type "Float (double-precision)") (InputAction :type "InputAction Object Reference" :default "/Game/ExternalAsset/VRTemplate/Input/Actions/IA_Shoot_Right.IA_Shoot_Right"))
  (:`Started`
    (if (`|EnumEquality` (`/Game/ExternalAsset/VRTemplate/Blueprints/GrabComponent.GetHeldByHand` (`self.GrabComponent`)) "Right")
      (goto _label))))

(event `self.GrabComponent.OnGrabbed`
  (`self.EnableInput` (`GameplayStatics.GetPlayerController` 0))
  (`EnhancedInputSubsystemInterface.AddMappingContext` (pcsubsystem `EnhancedInputLocalPlayerSubsystem` (`GameplayStatics.GetPlayerController` 0)) (select `bool` (`|EnumEquality` (`/Game/ExternalAsset/VRTemplate/Blueprints/GrabComponent.GetHeldByHand` (`self.GrabComponent`)) "Right") :`false` "/Game/ExternalAsset/VRTemplate/Input/IMC_Weapon_Left.IMC_Weapon_Left" :`true` "/Game/ExternalAsset/VRTemplate/Input/IMC_Weapon_Right.IMC_Weapon_Right" :!type "InputMappingContext Object Reference") 1 (struct)))

(event `self.GrabComponent.OnDropped`
  (`self.DisableInput` (`GameplayStatics.GetPlayerController` 0))
  (`EnhancedInputSubsystemInterface.RemoveMappingContext` (pcsubsystem `EnhancedInputLocalPlayerSubsystem` (`GameplayStatics.GetPlayerController` 0)) (select `bool` (`|EnumEquality` (`/Game/ExternalAsset/VRTemplate/Blueprints/GrabComponent.GetHeldByHand` (`self.GrabComponent`)) "Right") :`false` "/Game/ExternalAsset/VRTemplate/Input/IMC_Weapon_Left.IMC_Weapon_Left" :`true` "/Game/ExternalAsset/VRTemplate/Input/IMC_Weapon_Right.IMC_Weapon_Right" :!type "InputMappingContext Object Reference") (struct)))

(fn `UserConstructionScript`)